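; BP_Target is a target that awards score once and starts simulating physics on its mesh when hit.
; Its hit event casts the class of HitComponent, the target's own mesh rather than the other actor, to BP_2HWeapon, gating everything after it.
; Past that cast it prints the class name, then an IsHit flag limits AddScore on GM_MoveIt_Arthur and the physics switch to one run.
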(event OnComponentHit(SM_Target)
  (params (HitComponent :type Primitive%20Component%20Object%20Reference) (OtherActor :type Actor%20Object%20Reference) (OtherComp :type Primitive%20Component%20Object%20Reference) (NormalImpulse :type Vector :default "0, 0, 0") (Hit :type Hit%20Result%20Structure%20%28by%20ref%29))
  (bind _asbp_2hweapon (Utilities|Casting|CastToBP_2HWeaponClass (Utilities|GetClass HitComponent)))
  (Development|PrintString (Utilities|GetClassDisplayName _asbp_2hweapon))
  (if (not (Variables|Default|GetIsHit?))
    (Variables|Default|SetIsHit? true)
    (bind _asgm_move_it_arthur (Utilities|Casting|CastToGM_MoveIt_Arthur (Game|GetGameMode)))
    (Default|AddScore _asgm_move_it_arthur)
    (Physics|SetSimulatePhysics (Variables|Default|GetSM_Target) true)))

(fn ConstructionScript)